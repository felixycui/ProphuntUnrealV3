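; Game state for a hider-versus-seeker mode, holding the round timer, team counts and result.
; BeginPlay reads the timer from BP_GameplayGameMode and, on authority, counts both teams into it.
; Timer, count, kill and game-over updates chain through Client, Server and Multicast-named events; an empty team triggers EndGame on every BP_BaseCharacter.
; Separate events lock hider props and unfreeze seekers.
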(event `Lock Hiders`
  ;[1 1 1] lock hider props
  (bind _outactors (`GameplayStatics.GetAllActorsOfClass` "/Game/_Main/Characters/Hider.Hider_C"))
  (for _array_element _outactors
    (`/Game/_Main/Characters/Hider.Lock Prop` _array_element)))

(event `Unfreeze Seekers`
  ;[1 1 1] unfreeze seekers
  (bind _outactors (`GameplayStatics.GetAllActorsOfClass` "/Game/_Main/Characters/Seeker.Seeker_C"))
  (for _array_element _outactors
    (`/Game/_Main/Characters/Seeker.Unfreeze` _array_element)))

(event `self.ReceiveBeginPlay`
  ;[1 1 1] BeginPlay; initialize variables
  (bind _asbp_gameplay_game_mode (cast `/Game/_Main/Gameplay/BP_GameplayGameMode` (`GameplayStatics.GetGameMode`)))
  (`self.Set Minutes` (`/Game/_Main/Gameplay/BP_GameplayGameMode.Minutes Left` _asbp_gameplay_game_mode))
  (`self.Set Seconds` (`/Game/_Main/Gameplay/BP_GameplayGameMode.Seconds Left` _asbp_gameplay_game_mode))
  (`/Engine/EditorBlueprintResources/ActorMacros.Switch Has Authority`
    (:`Authority`
      (bind _outactors (`GameplayStatics.GetAllActorsOfClass` "/Game/_Main/Characters/Hider.Hider_C"))
      (bind _asbp_gameplay_game_mode_2 (cast `/Game/_Main/Gameplay/BP_GameplayGameMode` (`GameplayStatics.GetGameMode`)))
      (bind _returnvalue (`KismetArrayLibrary.Array_Length` _outactors))
      (bind _output_get (set `/Game/_Main/Gameplay/BP_GameplayGameMode.Num Hiders Alive` _returnvalue _asbp_gameplay_game_mode_2))
      (`KismetSystemLibrary.PrintString` (`KismetStringLibrary.Concat_StrStr` "num hiders: " (`KismetStringLibrary.Conv_IntToString` _returnvalue)))
      (bind _outactors_2 (`GameplayStatics.GetAllActorsOfClass` "/Game/_Main/Characters/Seeker.Seeker_C"))
      (bind _returnvalue_2 (`KismetArrayLibrary.Array_Length` _outactors_2))
      (bind _output_get_2 (set `/Game/_Main/Gameplay/BP_GameplayGameMode.Num Seekers Alive` _returnvalue_2 _asbp_gameplay_game_mode_2))
      (`KismetSystemLibrary.PrintString` (`KismetStringLibrary.Concat_StrStr` "num seekers: " (`KismetStringLibrary.Conv_IntToString` _returnvalue_2)))
      (set `/Game/_Main/Gameplay/BP_GameplayGameMode.NumPlayers` (+ _returnvalue _returnvalue_2) _asbp_gameplay_game_mode_2)
      (`self.Set Hiders Left` _output_get)
      (`self.Set Seekers Left` _output_get_2))))

(event `Set Seekers Left`
  (params (`num seekers` :type Integer))
  ;[1 1 1] Set Seekers Left
  (`self.Set Seekers Left Client` `num seekers`))

(event `Set Minutes`
  (params (minutes :type Integer))
  ;[1 1 1] Update Timer
  (`self.Set Minutes Client` minutes))

(event `Set Seconds`
  (params (seconds :type Integer))
  ;[1 1 1] Update Timer
  (`self.Set Seconds Client` seconds))

(event `Set Hiders Left`
  (params (`num hiders` :type Integer))
  ;[1 1 1] Set Hiders Left
  (`self.Set Hiders Left Cllient` `num hiders`))

(event `Set Minutes Client`
  (params (minutes :type Integer))
  ;[1 1 1] Update Timer
  (`self.Set Minutes Server` minutes))

(event `Set Seconds Client`
  (params (seconds :type Integer))
  ;[1 1 1] Update Timer
  (`self.Set Seconds Server` seconds))

(event `Set Seekers Left Client`
  (params (`num seekers` :type Integer))
  ;[1 1 1] Set Seekers Left
  (`self.Set Seekers Left Server` `num seekers`))

(event `Set Hiders Left Cllient`
  (params (`num hiders` :type Integer))
  ;[1 1 1] Set Hiders Left
  (`self.Set Hiders Left Server` `num hiders`))

(event `Set Seconds Server`
  (params (seconds :type Integer))
  ;[1 1 1] Update Timer
  (`self.Set Seconds Multicast` seconds))

(event `Set Minutes Server`
  (params (minutes :type Integer))
  ;[1 1 1] Update Timer
  (`self.Set Minutes Multicast` minutes))

(event `Set Hiders Left Server`
  (params (`num hiders` :type Integer))
  ;[1 1 1] Set Hiders Left
  (`self.Set Hiders Left Multicast` `num hiders`))

(event `Set Seekers Left Server`
  (params (`num seekers` :type Integer))
  ;[1 1 1] Set Seekers Left
  (`self.Set Seekers Left Multicast` `num seekers`))

(event `Set Minutes Multicast`
  (params (minutes :type Integer))
  ;[1 1 1] Update Timer
  (set `self.Minutes Left` minutes))

(event `Set Seconds Multicast`
  (params (seconds :type Integer))
  ;[1 1 1] Update Timer
  (set `self.Seconds Left` seconds))

(event `Set Seekers Left Multicast`
  (params (`num seekers` :type Integer))
  ;[1 1 1] Set Seekers Left
  (set `self.Num Seekers Left` `num seekers`))

(event `Set Hiders Left Multicast`
  (params (`num hiders` :type Integer))
  ;[1 1 1] Set Hiders Left
  (set `self.Num Hiders Left` `num hiders`))

(event `Kill Hider`
  ;[1 1 1] Kill Hider
  (`self.Kill Hider Client`))

(event `Kill Seeker`
  ;[1 1 1] Kill Seeker
  (`self.Kill Seeker Client`))

(event `End Game`
  (params (`Seekers Win` :type Boolean))
  ;[1 1 1] Game Over
  (`KismetSystemLibrary.PrintString` "GAME OVER")
  (`self.End Game Client` `Seekers Win`))

(event `Kill Hider Client`
  ;[1 1 1] Kill Hider
  (`self.Kill Hider Server`))

(event `Kill Seeker Client`
  ;[1 1 1] Kill Seeker
  (`self.Kill Seeker Server`))

(event `End Game Client`
  (params (`Seekers Win` :type Boolean))
  ;[1 1 1] Game Over
  (`self.End Game Server` `Seekers Win`))

(event `Kill Hider Server`
  ;[1 1 1] Kill Hider
  (`self.Kill Hider Multicast`))

(event `Kill Seeker Server`
  ;[1 1 1] Kill Seeker
  (`self.Kill Seeker Multicast`))

(event `End Game Server`
  (params (`Seekers Win` :type Boolean))
  ;[1 1 1] Game Over
  (`self.End Game Multicast` `Seekers Win`))

(event `Kill Hider Multicast`
  ;[1 1 1] Kill Hider
  (bind _output_get (set `self.Num Hiders Left` (`KismetMathLibrary.Max` (- (`self.Num Hiders Left`) 1))))
  (if (<= _output_get 0)
    (`self.End Game` true)))

(event `Kill Seeker Multicast`
  ;[1 1 1] Kill Seeker
  (bind _output_get (set `self.Num Seekers Left` (`KismetMathLibrary.Max` (- (`self.Num Seekers Left`) 1))))
  (if (<= _output_get 0)
    (`self.End Game` false)))

(event `End Game Multicast`
  (params (`Seekers Win` :type Boolean))
  ;[1 1 1] Game Over
  (set `self.Game Over` true)
  (set `self.Seekers Win` `Seekers Win`)
  (bind _outactors (`GameplayStatics.GetAllActorsOfClass` "/Game/_Main/Characters/BP_BaseCharacter.BP_BaseCharacter_C"))
  (for _array_element _outactors
    (`/Game/_Main/Characters/BP_BaseCharacter.End Game` _array_element))
  (`KismetSystemLibrary.PrintString` "MULTICAST GAME OVER"))

(fn `UserConstructionScript`)
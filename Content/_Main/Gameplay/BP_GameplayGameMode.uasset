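; Game mode for a multiplayer hider-versus-seeker prop game, running the match countdown, player spawning and chat relay.
; A one-second timer pushes time from the game instance's setting into BP_GameState and calls EndGame at zero.
; SpawnPlayer possesses the selected character at a random PlayerStart and tracks Hiders, which swap to prop meshes after all players join.
; Chat fans out to joined controllers, and logout triggers session destruction through the game instance.
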(event `self.ReceiveBeginPlay`
  ;[1 1 1] Begin play
  (bind _newparam (message `/Game/_Main/BPI_GameInstance.SteamGameInstanceRef` (`GameplayStatics.GetGameInstance`)))
  (bind _output_get (set `self.Minutes Left` (`/Game/_Main/SteamGameInstance.ServerTimeMinutes` _newparam)))
  (bind _asbp_game_state (cast `/Game/_Main/Lobby/BP_GameState` (`GameplayStatics.GetGameState`)))
  (`/Game/_Main/Lobby/BP_GameState.Set Minutes` _asbp_game_state _output_get)
  (bind _outactors (`GameplayStatics.GetAllActorsOfClass` "/Game/_Main/Characters/Hider.Hider_C"))
  (bind _returnvalue (`KismetArrayLibrary.Array_Length` _outactors))
  (set `self.Num Hiders Alive` _returnvalue)
  (`KismetSystemLibrary.K2_SetTimer` null "Update Timer" 1.0 (not (`self.Game Over`)))
  (bind _outactors_2 (`GameplayStatics.GetAllActorsOfClass` "/Game/_Main/Characters/Seeker.Seeker_C"))
  (set `self.NumPlayers` (+ _returnvalue (`KismetArrayLibrary.Array_Length` _outactors_2))))

(event `Update Timer`
  ;[1 1 1] Update timer
  (bind _output_get (set `self.Seconds Left` (- (`self.Seconds Left`) 1)))
  (`|ExecutionSequence`
    (:`then_0`
      (if (== _output_get -1)
        (set `self.Minutes Left` (- (`self.Minutes Left`) 1))
        (set `self.Seconds Left` 59)))
    (:`then_1`
      (bind _asbp_game_state (cast `/Game/_Main/Lobby/BP_GameState` (`GameplayStatics.GetGameState`)))
      (`/Game/_Main/Lobby/BP_GameState.Set Minutes` _asbp_game_state (`self.Minutes Left`))
      (`/Game/_Main/Lobby/BP_GameState.Set Seconds` _asbp_game_state (`self.Seconds Left`)))
    (:`then_2`
      (if (and (<= (`self.Minutes Left`) 0) (<= (`self.Seconds Left`) 0))
        (`KismetSystemLibrary.K2_ClearTimer` null "UpdateTimer")
        (bind _asbp_game_state_2 (cast `/Game/_Main/Lobby/BP_GameState` (`GameplayStatics.GetGameState`)))
        (`/Game/_Main/Lobby/BP_GameState.End Game` _asbp_game_state_2 (<= (`/Game/_Main/Lobby/BP_GameState.Num Hiders Left` _asbp_game_state_2) 0))))))

(event `SpawnPlayer`
  (params (PlayerController :type "PlayerController Object Reference") (SelectedCharacter :type "Character Class Reference"))
  (bind _returnvalue (`Controller.K2_GetPawn` PlayerController))
  (bind _spawnpoints (`self.SpawnPoints`))
  ;[1 1 1] Spawn Player at a random player spawn location
  (bind _outactors (`GameplayStatics.GetAllActorsOfClass` "/Script/Engine.PlayerStart"))
  (set `self.SpawnPoints` _outactors)
  (`/Engine/EditorBlueprintResources/StandardMacros.IsValid` _returnvalue
    (:`Is Valid`
      (`self.K2_DestroyActor` _returnvalue))
    (:`Is Not Valid`
      (bind _returnvalue_2 (`|SpawnActorFromClass` SelectedCharacter (`self.GetTransform` (`|GetArrayItem` _spawnpoints (`KismetMathLibrary.RandomIntegerInRange` 0 (- (`KismetArrayLibrary.Array_Length` _spawnpoints) 1)))) "Undefined" "OverrideRootScale" null null))
      (`Controller.Possess` PlayerController _returnvalue_2)
      (bind _gameplaypc (message `/Game/_Main/Gameplay/BPI_GameplayPC.GameplayPCref` (`GameplayStatics.GetPlayerController` 0)))
      (`/Game/_Main/Gameplay/BP_GameplayPC.SetCharacterObject` _gameplaypc _returnvalue_2)
      ;[1 1 1] Add the hider to the running list
      (if (== SelectedCharacter "/Game/_Main/Characters/Hider.Hider_C")
        (bind _ashider (cast `/Game/_Main/Characters/Hider` _returnvalue_2))
        (`KismetArrayLibrary.Array_Add` (`self.AllHiders`) _ashider)))))

(event `UpdateAllHiders`
  ;[1 0.1329 0.6916] After a 2 second delay from OnSwapPlayerControllers, updates all Hiders by hiding their default meshes and turning on their prop meshes
  (for _array_element (`self.AllHiders`)
    (`/Game/_Main/Characters/Hider.TurnOffDefaultMesh` _array_element)
    (`/Game/_Main/Characters/Hider.TurnOnPropMesh` _array_element)))

(event `self.K2_OnSwapPlayerControllers`
  (params (OldPC :type "PlayerController Object Reference") (NewPC :type "PlayerController Object Reference"))
  ;[1 1 1] When a player controller is swapped, this is called.  I also keep track of the number of connected players with this. No tthe best way but, it works i think.
  (`KismetArrayLibrary.Array_Add` (`self.AllPlayerControllers`) NewPC)
  (`KismetSystemLibrary.PrintString` "PlayerJoined!")
  (`/Engine/EditorBlueprintResources/StandardMacros.IncrementInt` (`self.NumPlayersJoinedSoFar`)
    (:`  `
      (bind _newparam (message `/Game/_Main/BPI_GameInstance.SteamGameInstanceRef` (`GameplayStatics.GetGameInstance`)))
      (if (== (`/Game/_Main/SteamGameInstance.MaxPlayers` _newparam) (`self.NumPlayersJoinedSoFar`))
        (`KismetSystemLibrary.PrintString` "All players joined!")
        (`KismetSystemLibrary.Delay` 2.0)
        (`self.UpdateAllHiders`)))))

(event `self.K2_OnLogout`
  (params (ExitingController :type "Controller Object Reference"))
  (bind _gameplaypc (message `/Game/_Main/Gameplay/BPI_GameplayPC.GameplayPCref` ExitingController))
  (bind _newparam (message `/Game/_Main/BPI_GameInstance.SteamGameInstanceRef` (`GameplayStatics.GetGameInstance`)))
  (message `/Game/_Main/BPI_GameInstance.DestroySessionCaller` _newparam _gameplaypc))

(event `UpdateChat`
  (params (Sender :type Text) (Chat :type Text))
  (for _array_element (`self.AllPlayerControllers`)
    (bind _gameplaypc (message `/Game/_Main/Gameplay/BPI_GameplayPC.GameplayPCref` _array_element))
    (`/Game/_Main/Gameplay/BP_GameplayPC.UpdateChatWindow` _gameplaypc Sender Chat)))

(fn `GameplayGMRef`
  (returns (GameplayGMRef :type "/Game/_Main/Gameplay/BP_GameplayGameMode Object Reference"))
  (return self))

(fn `UserConstructionScript`)
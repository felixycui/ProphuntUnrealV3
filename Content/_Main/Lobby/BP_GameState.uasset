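; Game state for a hide-and-seek match, tracking time left, remaining hiders and the game-over result.
; BeginPlay counts Hider actors and copies minutes and seconds from BP_GameplayGameMode.
; Time updates, hider kills and game end each pass through events named Client, Server and Multicast before changing state.
; When no hiders remain, seekers win and EndGame runs on every BP_BaseCharacter.
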(event `Set Minutes`
  (params (minutes :type Integer))
  ;[1 1 1] Update Timer
  (`self.Set Minutes Client` minutes))

(event `Set Seconds`
  (params (seconds :type Integer))
  ;[1 1 1] Update Timer
  (`self.Set Seconds Client` seconds))

(event `Set Minutes Client`
  (params (minutes :type Integer))
  ;[1 1 1] Update Timer
  (`self.Set Minutes Server` minutes))

(event `Set Seconds Client`
  (params (seconds :type Integer))
  ;[1 1 1] Update Timer
  (`self.Set Seconds Server` seconds))

(event `Set Seconds Server`
  (params (seconds :type Integer))
  ;[1 1 1] Update Timer
  (`self.Set Seconds Multicast` seconds))

(event `Set Minutes Server`
  (params (minutes :type Integer))
  ;[1 1 1] Update Timer
  (`self.Set Minutes Multicast` minutes))

(event `Set Minutes Multicast`
  (params (minutes :type Integer))
  ;[1 1 1] Update Timer
  (bind _output_get (set `self.Minutes Left` minutes))
  (`KismetSystemLibrary.PrintString` (`KismetStringLibrary.Concat_StrStr` "setting minutes to " (`KismetStringLibrary.Conv_IntToString` _output_get))))

(event `Set Seconds Multicast`
  (params (seconds :type Integer))
  ;[1 1 1] Update Timer
  (set `self.Seconds Left` seconds))

(event `self.ReceiveBeginPlay`
  (bind _outactors (`GameplayStatics.GetAllActorsOfClass` "/Game/_Main/Characters/Hider.Hider_C"))
  (set `self.Num Hiders Left` (`KismetArrayLibrary.Array_Length` _outactors))
  (bind _asbp_gameplay_game_mode (cast `/Game/_Main/Gameplay/BP_GameplayGameMode` (`GameplayStatics.GetGameMode`)))
  (`self.Set Minutes` (`/Game/_Main/Gameplay/BP_GameplayGameMode.Minutes Left` _asbp_gameplay_game_mode))
  (`self.Set Seconds` (`/Game/_Main/Gameplay/BP_GameplayGameMode.Seconds Left` _asbp_gameplay_game_mode)))

(event `Kill Hider`
  ;[1 1 1] Kill Hider
  (`self.Kill Hider Client`))

(event `End Game`
  (params (`Seekers Win` :type Boolean))
  ;[1 1 1] Game Over
  (`KismetSystemLibrary.PrintString` "GAME OVER")
  (`self.End Game Client` `Seekers Win`))

(event `Kill Hider Client`
  ;[1 1 1] Kill Hider
  (`self.Kill Hider Server`))

(event `End Game Client`
  (params (`Seekers Win` :type Boolean))
  ;[1 1 1] Game Over
  (`self.End Game Server` `Seekers Win`))

(event `Kill Hider Server`
  ;[1 1 1] Kill Hider
  (`self.Kill Hider Multicast`))

(event `End Game Server`
  (params (`Seekers Win` :type Boolean))
  ;[1 1 1] Game Over
  (`self.End Game Multicast` `Seekers Win`))

(event `Kill Hider Multicast`
  ;[1 1 1] Kill Hider
  (bind _output_get (set `self.Num Hiders Left` (- (`self.Num Hiders Left`) 1)))
  (if (<= _output_get 0)
    (`self.End Game` true)
    (`KismetSystemLibrary.PrintString` "SEEKERS WIN!!!")))

(event `End Game Multicast`
  (params (`Seekers Win` :type Boolean))
  ;[1 1 1] Game Over
  (set `self.Game Over` true)
  (set `self.Seekers Win` `Seekers Win`)
  (bind _outactors (`GameplayStatics.GetAllActorsOfClass` "/Game/_Main/Characters/BP_BaseCharacter.BP_BaseCharacter_C"))
  (for _array_element _outactors
    (`/Game/_Main/Characters/BP_BaseCharacter.End Game` _array_element))
  (`KismetSystemLibrary.PrintString` "MULTICAST GAME OVER"))

(fn `UserConstructionScript`)